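; Ranged enemy Blueprint that spawns a rifle on BeginPlay and attaches it to the mesh's right-hand socket.
; Attack plays the rifle shoot montage and signals attack end on completion or interruption.
; A montage notify checks for the base enemy AI controller, then line traces from the rifle to the enemy's own location.
; The shot is unfinished: it applies no damage, and its debug hit print sits behind a constant condition that never passes.
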(event `self.ReceiveBeginPlay`
  (`/Game/Enemies/AI/BPI_EnemyAI.EquipWeapon`))

(event `/Game/Enemies/AI/BPI_EnemyAI.EquipWeapon`
  (bind _returnvalue (`|SpawnActorFromClass` "/Game/Enemies/BP_Rifle.BP_Rifle_C" (`KismetMathLibrary.MakeTransform` (0.0 0.0 0.0)) "Undefined" "MultiplyWithRoot" null null))
  (bind _output_get (set `self.WeaponActor` _returnvalue))
  (`self.K2_AttachToComponent` _output_get (`self.Mesh`) "hand_r_rifle_Socket" "SnapToTarget" "SnapToTarget" "SnapToTarget" true)
  (set `self.IsEquippingWeapon` true))

(event `/Game/Enemies/AI/BPI_EnemyAI.Attack`
  (bind _notifyname (`|PlayMontage` (`self.Mesh`) "/Game/FirstPersonArms/Animations/FP_Rifle_Shoot_Montage.FP_Rifle_Shoot_Montage")
    (:`OnCompleted`
      (`self.OnAttackEnd` :!label _label))
    (:`OnInterrupted`
      (goto _label))
    (:`OnNotifyBegin`
      (switch `name` _notifyname
        (:`Default`
          (cast `/Game/Enemies/AI/AIC_Enemy_Base` (`AIBlueprintHelperLibrary.GetAIController` self))
          (`KismetSystemLibrary.LineTraceSingle` (`self.K2_GetActorLocation` (`self.WeaponActor`)) (`self.K2_GetActorLocation`) "TraceTypeQuery1")
          (if (not true)
            (`KismetSystemLibrary.PrintString` "Hit Target")))))))

(fn `UserConstructionScript`
  (`parent.UserConstructionScript`))