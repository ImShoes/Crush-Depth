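; Eel enemy that shoots electric projectiles and keeps its distance from the player's camera.
; Every tick it picks a range band: back away when close, face and fire at mid range, approach when farther, idle beyond that.
; Firing swaps static sprites for a flipbook during a delayed shot, then a timer resets the cooldown.
; On death, the killing weapon's actor tag selects a random pickup drop table.
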(event `self.ReceiveTick`
  (params (DeltaSeconds :type "Float (single-precision)"))
  (`self.Chase Player`))

(event `Chase Player`
  (bind _returnvalue (`GameplayStatics.GetPlayerCameraManager` 0))
  (bind _returnvalue_2 (`self.GetDistanceTo` _returnvalue))
  (bind _returnvalue_3 (`PlayerCameraManager.GetCameraLocation` _returnvalue))
  (bind _returnvalue_4 (`SceneComponent.K2_GetComponentLocation` (`self.CapsuleComponent`)))
  (bind _returnvalue_5 (`KismetMathLibrary.FindLookAtRotation` _returnvalue_4 _returnvalue_3))
  (bind _returnvalue_6 (- _returnvalue_4 _returnvalue_3))
  (if (and (<= _returnvalue_2 3000.0) (>= _returnvalue_2 1000.0))
    (`self.K2_SetActorRotation` self _returnvalue_5 false)
    (`self.fire`)
    (elif (<= _returnvalue_2 1000.0)
      (`self.AddMovementInput` self _returnvalue_6 1.0 false)
      (`KismetSystemLibrary.K2_PauseTimerHandle` (struct))
      (`self.K2_SetActorRotation` self _returnvalue_5 false :!label _label)
      (elif (and (<= _returnvalue_2 6000.0) (>= _returnvalue_2 3000.0))
        (`self.AddMovementInput` (* _returnvalue_6 (-1.0 -1.0 -1.0)))
        (`KismetSystemLibrary.K2_PauseTimerHandle` (struct))
        (goto _label)))))

(event `fire`
  (bind _returnvalue (`self.K2_GetActorRotation`))
  (bind _attackstate (`self.attackstate`))
  (bind _attackstate_2 (`self.attackstate`))
  (if (`self.canfire`)
    (set `self.canfire` false)
    (`PaperFlipbookComponent.SetPlayRate` (`self.PaperFlipbook`) 1.0)
    (set `self.attackstate` false)
    (`SceneComponent.SetVisibility` (`self.Sprite`) _attackstate false)
    (`SceneComponent.SetVisibility` (`self.PaperFlipbook`) (not _attackstate) false)
    (`SceneComponent.SetVisibility` (`self.back_eel_Sprite`) _attackstate false)
    (set `self.attackstate` true)
    (`KismetSystemLibrary.Delay` 1.0)
    (`|SpawnActorFromClass` "/Game/Enemies/bp_electricprojectile.bp_electricprojectile_C" (`KismetMathLibrary.MakeTransform` (+ (`self.K2_GetActorLocation`) (`KismetMathLibrary.GreaterGreater_VectorRotator` (200.0 0.0 0.0) _returnvalue)) _returnvalue) "Undefined" "MultiplyWithRoot" null null)
    (`KismetSystemLibrary.K2_SetTimer` null "timerdoine" 2.0)
    (`PaperFlipbookComponent.SetPlayRate` (`self.PaperFlipbook`) 0.0)
    (`SceneComponent.SetVisibility` (`self.Sprite`) _attackstate_2 false)
    (`SceneComponent.SetVisibility` (`self.PaperFlipbook`) (not _attackstate_2) false)
    (`SceneComponent.SetVisibility` (`self.back_eel_Sprite`) _attackstate_2 false)))

(event `self.ReceiveAnyDamage`
  (params (Damage :type "Float (single-precision)") (DamageType :type "DamageType Object Reference") (InstigatedBy :type "Controller Object Reference") (DamageCauser :type "Actor Object Reference"))
  (bind _output_get (set `self.health` (- (`self.health`) Damage)))
  (if (<= _output_get 0)
    (if (`self.ActorHasTag` DamageCauser "rebar")
      (`self.rebardeath`)
      (elif (`self.ActorHasTag` DamageCauser "nail")
        (`self.naildeath`)
        (elif (`self.ActorHasTag` DamageCauser "saw")
          (`self.sawdeath`)
          (elif (`self.ActorHasTag` DamageCauser "torch")
            (`self.Torchdeath`)))))
    (`self.K2_DestroyActor`)))

(fn `naildeath`
  (bind _returnvalue (`KismetMathLibrary.RandomIntegerInRange` 1 3))
  (bind _returnvalue_2 (`KismetMathLibrary.MakeTransform` (`self.K2_GetActorLocation`)))
  (if (> (`KismetMathLibrary.RandomFloatInRange` 0.0 100.0) 50.0)
    (`|SpawnActorFromClass` "/Game/FirstPerson/Blueprints/pickupitems/AirPickup.AirPickup_C" _returnvalue_2 "Undefined" "MultiplyWithRoot" null null))
  (if (> (`KismetMathLibrary.RandomFloatInRange` 0.0 100.0) 80.0)
    (if (== _returnvalue 1)
      (`|SpawnActorFromClass` "/Game/FirstPerson/Blueprints/pickupitems/RebarPickup.RebarPickup_C" _returnvalue_2 "Undefined" "MultiplyWithRoot" null null)
      (elif (== _returnvalue 2)
        (`|SpawnActorFromClass` "/Game/FirstPerson/Blueprints/pickupitems/NailPickup.NailPickup_C" _returnvalue_2 "Undefined" "MultiplyWithRoot" null null)
        (else
          (`|SpawnActorFromClass` "/Game/FirstPerson/Blueprints/pickupitems/SawPickup.SawPickup_C" _returnvalue_2 "Undefined" "MultiplyWithRoot" null null)))))
  (if (> (`KismetMathLibrary.RandomFloatInRange` 0.0 100.0) 75.0)
    (`|SpawnActorFromClass` "/Game/FirstPerson/Blueprints/pickupitems/HealthPickup.HealthPickup_C" _returnvalue_2 "Undefined" "MultiplyWithRoot" null null))
  (if (> (`KismetMathLibrary.RandomFloatInRange` 0.0 100.0) 65.0)
    (`|SpawnActorFromClass` "/Game/FirstPerson/Blueprints/pickupitems/NailPickup.NailPickup_C" _returnvalue_2 "Undefined" "MultiplyWithRoot" null null)))

(fn `rebardeath`
  (bind _returnvalue (`KismetMathLibrary.RandomIntegerInRange` 1 3))
  (bind _returnvalue_2 (`KismetMathLibrary.MakeTransform` (`self.K2_GetActorLocation`)))
  (if (> (`KismetMathLibrary.RandomFloatInRange` 0.0 100.0) 50.0)
    (`|SpawnActorFromClass` "/Game/FirstPerson/Blueprints/pickupitems/AirPickup.AirPickup_C" _returnvalue_2 "Undefined" "MultiplyWithRoot" null null))
  (if (> (`KismetMathLibrary.RandomFloatInRange` 0.0 100.0) 75.0)
    (if (== _returnvalue 1)
      (`|SpawnActorFromClass` "/Game/FirstPerson/Blueprints/pickupitems/RebarPickup.RebarPickup_C" _returnvalue_2 "Undefined" "MultiplyWithRoot" null null)
      (elif (== _returnvalue 2)
        (`|SpawnActorFromClass` "/Game/FirstPerson/Blueprints/pickupitems/NailPickup.NailPickup_C" _returnvalue_2 "Undefined" "MultiplyWithRoot" null null)
        (else
          (`|SpawnActorFromClass` "/Game/FirstPerson/Blueprints/pickupitems/SawPickup.SawPickup_C" _returnvalue_2 "Undefined" "MultiplyWithRoot" null null)))))
  (if (> (`KismetMathLibrary.RandomFloatInRange` 0.0 100.0) 75.0)
    (`|SpawnActorFromClass` "/Game/FirstPerson/Blueprints/pickupitems/HealthPickup.HealthPickup_C" _returnvalue_2 "Undefined" "MultiplyWithRoot" null null))
  (if (> (`KismetMathLibrary.RandomFloatInRange` 0.0 100.0) 60.0)
    (`|SpawnActorFromClass` "/Game/FirstPerson/Blueprints/pickupitems/RebarPickup.RebarPickup_C" _returnvalue_2 "Undefined" "MultiplyWithRoot" null null)))

(fn `sawdeath`
  (bind _returnvalue (`KismetMathLibrary.RandomIntegerInRange` 1 3))
  (bind _returnvalue_2 (`KismetMathLibrary.MakeTransform` (`self.K2_GetActorLocation`)))
  (if (> (`KismetMathLibrary.RandomFloatInRange` 0.0 100.0) 50.0)
    (`|SpawnActorFromClass` "/Game/FirstPerson/Blueprints/pickupitems/AirPickup.AirPickup_C" _returnvalue_2 "Undefined" "MultiplyWithRoot" null null))
  (if (> (`KismetMathLibrary.RandomFloatInRange` 0.0 100.0) 85.0)
    (if (== _returnvalue 1)
      (`|SpawnActorFromClass` "/Game/FirstPerson/Blueprints/pickupitems/RebarPickup.RebarPickup_C" _returnvalue_2 "Undefined" "MultiplyWithRoot" null null)
      (elif (== _returnvalue 2)
        (`|SpawnActorFromClass` "/Game/FirstPerson/Blueprints/pickupitems/NailPickup.NailPickup_C" _returnvalue_2 "Undefined" "MultiplyWithRoot" null null)
        (else
          (`|SpawnActorFromClass` "/Game/FirstPerson/Blueprints/pickupitems/SawPickup.SawPickup_C" _returnvalue_2 "Undefined" "MultiplyWithRoot" null null)))))
  (if (> (`KismetMathLibrary.RandomFloatInRange` 0.0 100.0) 80.0)
    (`|SpawnActorFromClass` "/Game/FirstPerson/Blueprints/pickupitems/HealthPickup.HealthPickup_C" _returnvalue_2 "Undefined" "MultiplyWithRoot" null null))
  (if (> (`KismetMathLibrary.RandomFloatInRange` 0.0 100.0) 70.0)
    (`|SpawnActorFromClass` "/Game/FirstPerson/Blueprints/pickupitems/SawPickup.SawPickup_C" _returnvalue_2 "Undefined" "MultiplyWithRoot" null null)))

(fn `timerdoine`
  (set `self.canfire` true))

(fn `Torchdeath`
  (bind _returnvalue (`KismetMathLibrary.RandomIntegerInRange` 1 3))
  (bind _returnvalue_2 (`KismetMathLibrary.MakeTransform` (`self.K2_GetActorLocation`)))
  (`|SpawnActorFromClass` "/Game/FirstPerson/Blueprints/pickupitems/AirPickup.AirPickup_C" _returnvalue_2 "Undefined" "MultiplyWithRoot" null null)
  (if (> (`KismetMathLibrary.RandomFloatInRange` 0.0 100.0) 60.0)
    (if (== _returnvalue 1)
      (`|SpawnActorFromClass` "/Game/FirstPerson/Blueprints/pickupitems/RebarPickup.RebarPickup_C" _returnvalue_2 "Undefined" "MultiplyWithRoot" null null)
      (elif (== _returnvalue 2)
        (`|SpawnActorFromClass` "/Game/FirstPerson/Blueprints/pickupitems/NailPickup.NailPickup_C" _returnvalue_2 "Undefined" "MultiplyWithRoot" null null)
        (else
          (`|SpawnActorFromClass` "/Game/FirstPerson/Blueprints/pickupitems/SawPickup.SawPickup_C" _returnvalue_2 "Undefined" "MultiplyWithRoot" null null)))))
  (if (> (`KismetMathLibrary.RandomFloatInRange` 0.0 100.0) 75.0)
    (`|SpawnActorFromClass` "/Game/FirstPerson/Blueprints/pickupitems/HealthPickup.HealthPickup_C" _returnvalue_2 "Undefined" "MultiplyWithRoot" null null)))

(fn `UserConstructionScript`)