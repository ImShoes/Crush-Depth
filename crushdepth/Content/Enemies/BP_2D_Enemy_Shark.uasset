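; 2D sprite shark enemy that swims toward the player camera within range and bites when the player overlaps its AttackBox.
; Tick drives ChasePlayer, which re-calls itself after a Delay; Attack swaps flipbook visibility and subtracts player health directly.
; Boosting raises swim speed and aims a Niagara beam at the supplied actor.
; Lethal damage selects a randomized pickup-drop function by the damage causer's weapon tag, then destroys the shark.
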(event `self.ReceiveTick`
  (params (DeltaSeconds :type "Float (single-precision)"))
  (bind _niagara (`self.Niagara`))
  (if (`self.boosted?`)
    (`NiagaraComponent.SetVariableVec3` _niagara "Beam End" (`self.K2_GetActorLocation` (stale `boosted` NewParam2)))
    (else
      (`NiagaraComponent.SetVariableVec3` _niagara "Beam End" (`self.K2_GetActorLocation`))))
  (if (`self.Is Shark Enemy Dead?`)
    _
    (elif (`self.Is Enemy Attacking?`)
      (if (== (`PaperFlipbookComponent.GetPlaybackPositionInFrames` (`self.Sprite`)) 3)
        (`/Engine/EditorBlueprintResources/StandardMacros.DoOnce` false
          (:`Completed`
            (`self.HitCheck`))))
      (else
        (`self.Chase Player`)))))

(event `Animation Update`
  (`PaperFlipbookComponent.SetFlipbook` (`self.Sprite`) (select `bool` (> (`KismetMathLibrary.VSize` (`MovementComponent.Velocity` (`self.CharacterMovement`))) 0.0) :`false` "/Game/Enemies/AI/Art/EnemyAI_Idle_Walk_Flipbook.EnemyAI_Idle_Walk_Flipbook" :`true` "/Game/Enemies/AI/Art/EnemyAI_Idle_Walk_Flipbook.EnemyAI_Idle_Walk_Flipbook" :!type "PaperFlipbook Object Reference")))

(event `Chase Player`
  (bind _returnvalue (`GameplayStatics.GetPlayerCameraManager` 0))
  (bind _returnvalue_2 (`PlayerCameraManager.GetCameraLocation` _returnvalue))
  (bind _returnvalue_3 (`SceneComponent.K2_GetComponentLocation` (`self.CapsuleComponent`)))
  (if (<= (`self.GetDistanceTo` _returnvalue) 4000.0)
    (`self.AddMovementInput` self (* (- _returnvalue_3 _returnvalue_2) (-1.0 -1.0 -1.0)) 1.0 false)
    (`self.K2_SetActorRotation` self (`KismetMathLibrary.FindLookAtRotation` _returnvalue_3 _returnvalue_2) false)
    (`KismetSystemLibrary.Delay` 0.5)
    (`self.Chase Player`)
    (if (`self.closeenough`)
      (`self.Attack`))))

(event `Attack`
  (bind _attackstate (`self.attackstate`))
  (bind _attackstate_2 (`self.attackstate`))
  (`PaperFlipbookComponent.SetPlayRate` (`self.PaperFlipbook`) 1.0)
  (set `self.attackstate` false)
  (`SceneComponent.SetVisibility` (`self.Sprite`) _attackstate false)
  (`SceneComponent.SetVisibility` (`self.PaperFlipbook`) (not _attackstate) false)
  (`SceneComponent.SetVisibility` (`self.back_Sprite`) _attackstate false)
  (set `self.attackstate` true)
  (bind _asbp_first_person_character (cast `/Game/FirstPerson/Blueprints/BP_FirstPersonCharacter` (`GameplayStatics.GetPlayerCharacter` 0)))
  (set `/Game/FirstPerson/Blueprints/BP_FirstPersonCharacter.heath` (- (`/Game/FirstPerson/Blueprints/BP_FirstPersonCharacter.heath` _asbp_first_person_character) 7) _asbp_first_person_character)
  (`KismetSystemLibrary.Delay` 0.5)
  (`PaperFlipbookComponent.SetPlayRate` (`self.PaperFlipbook`) 0.0)
  (`SceneComponent.SetVisibility` (`self.Sprite`) _attackstate_2 false)
  (`SceneComponent.SetVisibility` (`self.PaperFlipbook`) (not _attackstate_2) false)
  (`SceneComponent.SetVisibility` (`self.back_Sprite`) _attackstate_2 false))

(event `boosted`
  (params (NewParam2 :type "/Game/Enemies/BP_2D_Enemy_Lobster Object Reference"))
  (set `CharacterMovementComponent.MaxSwimSpeed` 600.0 (`self.CharacterMovement`))
  (set `self.boosted?` true))

(event `unboosted`
  (set `CharacterMovementComponent.MaxSwimSpeed` 300.0 (`self.CharacterMovement`))
  (set `self.boosted?` false))

(event `self.AttackBox.OnComponentBeginOverlap`
  (params (OverlappedComponent :type "PrimitiveComponent Object Reference") (OtherActor :type "Actor Object Reference") (OtherComp :type "PrimitiveComponent Object Reference") (OtherBodyIndex :type Integer) (bFromSweep :type Boolean) (SweepResult :type "HitResult Structure (by ref)"))
  (cast `/Game/FirstPerson/Blueprints/BP_FirstPersonCharacter` OtherActor)
  (set `self.closeenough` true))

(event `self.AttackBox.OnComponentEndOverlap`
  (params (OverlappedComponent :type "PrimitiveComponent Object Reference") (OtherActor :type "Actor Object Reference") (OtherComp :type "PrimitiveComponent Object Reference") (OtherBodyIndex :type Integer))
  (cast `/Game/FirstPerson/Blueprints/BP_FirstPersonCharacter` OtherActor)
  (set `self.closeenough` false))

(event `self.ReceiveAnyDamage`
  (params (Damage :type "Float (single-precision)") (DamageType :type "DamageType Object Reference") (InstigatedBy :type "Controller Object Reference") (DamageCauser :type "Actor Object Reference"))
  (bind _output_get (set `self.health` (- (`self.health`) Damage)))
  (if (<= _output_get 0)
    (if (`self.ActorHasTag` DamageCauser "rebar")
      (`self.rebardeath`)
      (elif (`self.ActorHasTag` DamageCauser "nail")
        (`self.naildeath`)
        (elif (`self.ActorHasTag` DamageCauser "saw")
          (`self.sawdeath`)
          (elif (`self.ActorHasTag` DamageCauser "torch")
            (`self.torchdeath`)))))
    (`self.K2_DestroyActor`)))

(fn `HitCheck`
  (for _array_element (`PrimitiveComponent.GetOverlappingActors` (`self.AttackBox`) "BP_2D_Enemy_Shark_C")
    (if (!= _array_element self)
      (`GameplayStatics.ApplyDamage` _array_element (`self.DamageAmount`)))))

(fn `naildeath`
  (bind _returnvalue (`KismetMathLibrary.RandomIntegerInRange` 1 3))
  (bind _returnvalue_2 (`KismetMathLibrary.MakeTransform` (`self.K2_GetActorLocation`)))
  (if (> (`KismetMathLibrary.RandomFloatInRange` 0.0 100.0) 50.0)
    (`|SpawnActorFromClass` "/Game/FirstPerson/Blueprints/pickupitems/AirPickup.AirPickup_C" _returnvalue_2 "Undefined" "MultiplyWithRoot" null null))
  (if (> (`KismetMathLibrary.RandomFloatInRange` 0.0 100.0) 80.0)
    (if (== _returnvalue 1)
      (`|SpawnActorFromClass` "/Game/FirstPerson/Blueprints/pickupitems/RebarPickup.RebarPickup_C" _returnvalue_2 "Undefined" "MultiplyWithRoot" null null)
      (elif (== _returnvalue 2)
        (`|SpawnActorFromClass` "/Game/FirstPerson/Blueprints/pickupitems/NailPickup.NailPickup_C" _returnvalue_2 "Undefined" "MultiplyWithRoot" null null)
        (else
          (`|SpawnActorFromClass` "/Game/FirstPerson/Blueprints/pickupitems/SawPickup.SawPickup_C" _returnvalue_2 "Undefined" "MultiplyWithRoot" null null)))))
  (if (> (`KismetMathLibrary.RandomFloatInRange` 0.0 100.0) 75.0)
    (`|SpawnActorFromClass` "/Game/FirstPerson/Blueprints/pickupitems/HealthPickup.HealthPickup_C" _returnvalue_2 "Undefined" "MultiplyWithRoot" null null))
  (if (> (`KismetMathLibrary.RandomFloatInRange` 0.0 100.0) 65.0)
    (`|SpawnActorFromClass` "/Game/FirstPerson/Blueprints/pickupitems/NailPickup.NailPickup_C" _returnvalue_2 "Undefined" "MultiplyWithRoot" null null)))

(fn `rebardeath`
  (bind _returnvalue (`KismetMathLibrary.RandomIntegerInRange` 1 3))
  (bind _returnvalue_2 (`KismetMathLibrary.MakeTransform` (`self.K2_GetActorLocation`)))
  (if (> (`KismetMathLibrary.RandomFloatInRange` 0.0 100.0) 50.0)
    (`|SpawnActorFromClass` "/Game/FirstPerson/Blueprints/pickupitems/AirPickup.AirPickup_C" _returnvalue_2 "Undefined" "MultiplyWithRoot" null null))
  (if (> (`KismetMathLibrary.RandomFloatInRange` 0.0 100.0) 75.0)
    (if (== _returnvalue 1)
      (`|SpawnActorFromClass` "/Game/FirstPerson/Blueprints/pickupitems/RebarPickup.RebarPickup_C" _returnvalue_2 "Undefined" "MultiplyWithRoot" null null)
      (elif (== _returnvalue 2)
        (`|SpawnActorFromClass` "/Game/FirstPerson/Blueprints/pickupitems/NailPickup.NailPickup_C" _returnvalue_2 "Undefined" "MultiplyWithRoot" null null)
        (else
          (`|SpawnActorFromClass` "/Game/FirstPerson/Blueprints/pickupitems/SawPickup.SawPickup_C" _returnvalue_2 "Undefined" "MultiplyWithRoot" null null)))))
  (if (> (`KismetMathLibrary.RandomFloatInRange` 0.0 100.0) 75.0)
    (`|SpawnActorFromClass` "/Game/FirstPerson/Blueprints/pickupitems/HealthPickup.HealthPickup_C" _returnvalue_2 "Undefined" "MultiplyWithRoot" null null))
  (if (> (`KismetMathLibrary.RandomFloatInRange` 0.0 100.0) 60.0)
    (`|SpawnActorFromClass` "/Game/FirstPerson/Blueprints/pickupitems/RebarPickup.RebarPickup_C" _returnvalue_2 "Undefined" "MultiplyWithRoot" null null)))

(fn `RestartAnim`
  (`PaperFlipbookComponent.SetLooping` (`self.Sprite`) true)
  (if (not (`PaperFlipbookComponent.IsPlaying` (`self.Sprite`)))
    (`PaperFlipbookComponent.Play` (`self.Sprite`))))

(fn `sawdeath`
  (bind _returnvalue (`KismetMathLibrary.RandomIntegerInRange` 1 3))
  (bind _returnvalue_2 (`KismetMathLibrary.MakeTransform` (`self.K2_GetActorLocation`)))
  (if (> (`KismetMathLibrary.RandomFloatInRange` 0.0 100.0) 50.0)
    (`|SpawnActorFromClass` "/Game/FirstPerson/Blueprints/pickupitems/AirPickup.AirPickup_C" _returnvalue_2 "Undefined" "MultiplyWithRoot" null null))
  (if (> (`KismetMathLibrary.RandomFloatInRange` 0.0 100.0) 85.0)
    (if (== _returnvalue 1)
      (`|SpawnActorFromClass` "/Game/FirstPerson/Blueprints/pickupitems/RebarPickup.RebarPickup_C" _returnvalue_2 "Undefined" "MultiplyWithRoot" null null)
      (elif (== _returnvalue 2)
        (`|SpawnActorFromClass` "/Game/FirstPerson/Blueprints/pickupitems/NailPickup.NailPickup_C" _returnvalue_2 "Undefined" "MultiplyWithRoot" null null)
        (else
          (`|SpawnActorFromClass` "/Game/FirstPerson/Blueprints/pickupitems/SawPickup.SawPickup_C" _returnvalue_2 "Undefined" "MultiplyWithRoot" null null)))))
  (if (> (`KismetMathLibrary.RandomFloatInRange` 0.0 100.0) 80.0)
    (`|SpawnActorFromClass` "/Game/FirstPerson/Blueprints/pickupitems/HealthPickup.HealthPickup_C" _returnvalue_2 "Undefined" "MultiplyWithRoot" null null))
  (if (> (`KismetMathLibrary.RandomFloatInRange` 0.0 100.0) 70.0)
    (`|SpawnActorFromClass` "/Game/FirstPerson/Blueprints/pickupitems/SawPickup.SawPickup_C" _returnvalue_2 "Undefined" "MultiplyWithRoot" null null)))

(fn `torchdeath`
  (bind _returnvalue (`KismetMathLibrary.RandomIntegerInRange` 1 3))
  (bind _returnvalue_2 (`KismetMathLibrary.MakeTransform` (`self.K2_GetActorLocation`)))
  (`|SpawnActorFromClass` "/Game/FirstPerson/Blueprints/pickupitems/AirPickup.AirPickup_C" _returnvalue_2 "Undefined" "MultiplyWithRoot" null null)
  (if (> (`KismetMathLibrary.RandomFloatInRange` 0.0 100.0) 60.0)
    (if (== _returnvalue 1)
      (`|SpawnActorFromClass` "/Game/FirstPerson/Blueprints/pickupitems/RebarPickup.RebarPickup_C" _returnvalue_2 "Undefined" "MultiplyWithRoot" null null)
      (elif (== _returnvalue 2)
        (`|SpawnActorFromClass` "/Game/FirstPerson/Blueprints/pickupitems/NailPickup.NailPickup_C" _returnvalue_2 "Undefined" "MultiplyWithRoot" null null)
        (else
          (`|SpawnActorFromClass` "/Game/FirstPerson/Blueprints/pickupitems/SawPickup.SawPickup_C" _returnvalue_2 "Undefined" "MultiplyWithRoot" null null)))))
  (if (> (`KismetMathLibrary.RandomFloatInRange` 0.0 100.0) 75.0)
    (`|SpawnActorFromClass` "/Game/FirstPerson/Blueprints/pickupitems/HealthPickup.HealthPickup_C" _returnvalue_2 "Undefined" "MultiplyWithRoot" null null)))

(fn `UserConstructionScript`)