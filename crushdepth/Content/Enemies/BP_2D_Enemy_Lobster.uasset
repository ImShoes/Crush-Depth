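; Lobster enemy with 2D sprites that hunts and melees the player and boosts Shark enemies inside its sphere.
; A looping timer moves it toward a nearby player at its own height, then triggers a cooldown-limited flipbook attack that damages whoever remains in AttackBox.
; Weapon tags on the damage causer scale damage taken and choose the death function, each rolling different pickup drops before the actor is destroyed.
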(event `self.Sphere.OnComponentBeginOverlap`
  (params (OverlappedComponent :type "PrimitiveComponent Object Reference") (OtherActor :type "Actor Object Reference") (OtherComp :type "PrimitiveComponent Object Reference") (OtherBodyIndex :type Integer) (bFromSweep :type Boolean) (SweepResult :type "HitResult Structure (by ref)"))
  (bind _asbp_2d_enemy_shark (cast `/Game/Enemies/BP_2D_Enemy_Shark` OtherActor))
  (set `self.is boosting?` true)
  (`/Game/Enemies/BP_2D_Enemy_Shark.boosted` _asbp_2d_enemy_shark self))

(event `self.Sphere.OnComponentEndOverlap`
  (params (OverlappedComponent :type "PrimitiveComponent Object Reference") (OtherActor :type "Actor Object Reference") (OtherComp :type "PrimitiveComponent Object Reference") (OtherBodyIndex :type Integer))
  (bind _asbp_2d_enemy_shark (cast `/Game/Enemies/BP_2D_Enemy_Shark` OtherActor))
  (set `self.is boosting?` false)
  (`/Game/Enemies/BP_2D_Enemy_Shark.unboosted` _asbp_2d_enemy_shark))

(event `self.ReceiveBeginPlay`
  (`KismetSystemLibrary.K2_SetTimerDelegate` (delegate `ChasePlayer`) 0.5 true))

(event `self.ReceiveTick`
  (params (DeltaSeconds :type "Float (single-precision)")))

(event `ChasePlayer`
  (if (<= (`self.GetDistanceTo` (`GameplayStatics.GetPlayerCameraManager` 0)) 5000.0)
    (`|AIMoveTo` self (`KismetMathLibrary.MakeVector` (.x (`SceneComponent.K2_GetComponentLocation` (`Character.CapsuleComponent` (`GameplayStatics.GetPlayerCharacter` 0)))) (.y (`SceneComponent.K2_GetComponentLocation` (`Character.CapsuleComponent` (`GameplayStatics.GetPlayerCharacter` 0)))) (.z (`SceneComponent.K2_GetComponentLocation` (`self.CapsuleComponent`)))) null 15.0
      (:`then`
        (if (`self.closeenough`)
          (`self.Attack`))))))

(event `Attack`
  (bind _attackstate (`self.attackstate`))
  (bind _attackstate_2 (`self.attackstate`))
  (if (`self.canattack`)
    (set `self.canattack` false)
    (`KismetSystemLibrary.K2_SetTimer` null "cooldown" 1.0)
    (`PaperFlipbookComponent.SetPlayRate` (`self.PaperFlipbook`) 1.0)
    (set `self.attackstate` false)
    (`SceneComponent.SetVisibility` (`self.Sprite`) _attackstate false)
    (`SceneComponent.SetVisibility` (`self.PaperFlipbook`) (not _attackstate) false)
    (`SceneComponent.SetVisibility` (`self.Back_lobster_Sprite`) _attackstate false)
    (bind _asbp_first_person_character (cast `/Game/FirstPerson/Blueprints/BP_FirstPersonCharacter` (`GameplayStatics.GetPlayerCharacter` 0)))
    (`KismetSystemLibrary.Delay` 0.5)
    (if (`self.closeenough`)
      (set `/Game/FirstPerson/Blueprints/BP_FirstPersonCharacter.heath` (- (`/Game/FirstPerson/Blueprints/BP_FirstPersonCharacter.heath` _asbp_first_person_character) 30) _asbp_first_person_character))
    (`KismetSystemLibrary.Delay` 0.5)
    (`PaperFlipbookComponent.SetPlayRate` (`self.PaperFlipbook`) 0.0)
    (set `self.attackstate` true)
    (`SceneComponent.SetVisibility` (`self.Sprite`) _attackstate_2 false)
    (`SceneComponent.SetVisibility` (`self.PaperFlipbook`) (not _attackstate_2) false)
    (`SceneComponent.SetVisibility` (`self.Back_lobster_Sprite`) _attackstate_2 false)))

(event `self.AttackBox.OnComponentBeginOverlap`
  (params (OverlappedComponent :type "PrimitiveComponent Object Reference") (OtherActor :type "Actor Object Reference") (OtherComp :type "PrimitiveComponent Object Reference") (OtherBodyIndex :type Integer) (bFromSweep :type Boolean) (SweepResult :type "HitResult Structure (by ref)"))
  (cast `/Game/FirstPerson/Blueprints/BP_FirstPersonCharacter` OtherActor)
  (set `self.closeenough` true))

(event `self.AttackBox.OnComponentEndOverlap`
  (params (OverlappedComponent :type "PrimitiveComponent Object Reference") (OtherActor :type "Actor Object Reference") (OtherComp :type "PrimitiveComponent Object Reference") (OtherBodyIndex :type Integer))
  (cast `/Game/FirstPerson/Blueprints/BP_FirstPersonCharacter` OtherActor)
  (set `self.closeenough` false))

(event `self.ReceiveAnyDamage`
  (params (Damage :type "Float (single-precision)") (DamageType :type "DamageType Object Reference") (InstigatedBy :type "Controller Object Reference") (DamageCauser :type "Actor Object Reference"))
  (if (`self.ActorHasTag` DamageCauser "rebar")
    (set `self.health` (- (`self.health`) (* Damage 0.75)))
    (if (<= (`self.health`) 0) :!label _label
      (if (`self.ActorHasTag` DamageCauser "rebar")
        (`self.rebardeath`)
        (elif (`self.ActorHasTag` DamageCauser "nail")
          (`self.naildeath`)
          (elif (`self.ActorHasTag` DamageCauser "saw")
            (`self.sawdeath`)
            (elif (`self.ActorHasTag` DamageCauser "torch")
              (`self.torchdeath`)))))
      (`self.K2_DestroyActor`))
    (elif (`self.ActorHasTag` DamageCauser "nail")
      (set `self.health` (- (`self.health`) (* Damage 0.5)))
      (goto _label)
      (elif (`self.ActorHasTag` DamageCauser "saw")
        (set `self.health` (- (`self.health`) Damage) :!label _label_2)
        (goto _label)
        (elif (`self.ActorHasTag` DamageCauser "torch")
          (goto _label_2))))))

(fn `cooldown`
  (set `self.canattack` true))

(fn `naildeath`
  (bind _returnvalue (`KismetMathLibrary.RandomIntegerInRange` 1 3))
  (bind _returnvalue_2 (`KismetMathLibrary.MakeTransform` (`self.K2_GetActorLocation`)))
  (if (> (`KismetMathLibrary.RandomFloatInRange` 0.0 100.0) 50.0)
    (`|SpawnActorFromClass` "/Game/FirstPerson/Blueprints/pickupitems/AirPickup.AirPickup_C" _returnvalue_2 "Undefined" "MultiplyWithRoot" null null))
  (if (> (`KismetMathLibrary.RandomFloatInRange` 0.0 100.0) 80.0)
    (if (== _returnvalue 1)
      (`|SpawnActorFromClass` "/Game/FirstPerson/Blueprints/pickupitems/RebarPickup.RebarPickup_C" _returnvalue_2 "Undefined" "MultiplyWithRoot" null null)
      (elif (== _returnvalue 2)
        (`|SpawnActorFromClass` "/Game/FirstPerson/Blueprints/pickupitems/NailPickup.NailPickup_C" _returnvalue_2 "Undefined" "MultiplyWithRoot" null null)
        (else
          (`|SpawnActorFromClass` "/Game/FirstPerson/Blueprints/pickupitems/SawPickup.SawPickup_C" _returnvalue_2 "Undefined" "MultiplyWithRoot" null null)))))
  (if (> (`KismetMathLibrary.RandomFloatInRange` 0.0 100.0) 75.0)
    (`|SpawnActorFromClass` "/Game/FirstPerson/Blueprints/pickupitems/HealthPickup.HealthPickup_C" _returnvalue_2 "Undefined" "MultiplyWithRoot" null null))
  (if (> (`KismetMathLibrary.RandomFloatInRange` 0.0 100.0) 65.0)
    (`|SpawnActorFromClass` "/Game/FirstPerson/Blueprints/pickupitems/NailPickup.NailPickup_C" _returnvalue_2 "Undefined" "MultiplyWithRoot" null null)))

(fn `NewFunction`
  (`KismetSystemLibrary.PrintString` "Hello"))

(fn `rebardeath`
  (bind _returnvalue (`KismetMathLibrary.RandomIntegerInRange` 1 3))
  (bind _returnvalue_2 (`KismetMathLibrary.MakeTransform` (`self.K2_GetActorLocation`)))
  (if (> (`KismetMathLibrary.RandomFloatInRange` 0.0 100.0) 50.0)
    (`|SpawnActorFromClass` "/Game/FirstPerson/Blueprints/pickupitems/AirPickup.AirPickup_C" _returnvalue_2 "Undefined" "MultiplyWithRoot" null null))
  (if (> (`KismetMathLibrary.RandomFloatInRange` 0.0 100.0) 75.0)
    (if (== _returnvalue 1)
      (`|SpawnActorFromClass` "/Game/FirstPerson/Blueprints/pickupitems/RebarPickup.RebarPickup_C" _returnvalue_2 "Undefined" "MultiplyWithRoot" null null)
      (elif (== _returnvalue 2)
        (`|SpawnActorFromClass` "/Game/FirstPerson/Blueprints/pickupitems/NailPickup.NailPickup_C" _returnvalue_2 "Undefined" "MultiplyWithRoot" null null)
        (else
          (`|SpawnActorFromClass` "/Game/FirstPerson/Blueprints/pickupitems/SawPickup.SawPickup_C" _returnvalue_2 "Undefined" "MultiplyWithRoot" null null)))))
  (if (> (`KismetMathLibrary.RandomFloatInRange` 0.0 100.0) 75.0)
    (`|SpawnActorFromClass` "/Game/FirstPerson/Blueprints/pickupitems/HealthPickup.HealthPickup_C" _returnvalue_2 "Undefined" "MultiplyWithRoot" null null))
  (if (> (`KismetMathLibrary.RandomFloatInRange` 0.0 100.0) 60.0)
    (`|SpawnActorFromClass` "/Game/FirstPerson/Blueprints/pickupitems/RebarPickup.RebarPickup_C" _returnvalue_2 "Undefined" "MultiplyWithRoot" null null)))

(fn `sawdeath`
  (bind _returnvalue (`KismetMathLibrary.RandomIntegerInRange` 1 3))
  (bind _returnvalue_2 (`KismetMathLibrary.MakeTransform` (`self.K2_GetActorLocation`)))
  (if (> (`KismetMathLibrary.RandomFloatInRange` 0.0 100.0) 50.0)
    (`|SpawnActorFromClass` "/Game/FirstPerson/Blueprints/pickupitems/AirPickup.AirPickup_C" _returnvalue_2 "Undefined" "MultiplyWithRoot" null null))
  (if (> (`KismetMathLibrary.RandomFloatInRange` 0.0 100.0) 85.0)
    (if (== _returnvalue 1)
      (`|SpawnActorFromClass` "/Game/FirstPerson/Blueprints/pickupitems/RebarPickup.RebarPickup_C" _returnvalue_2 "Undefined" "MultiplyWithRoot" null null)
      (elif (== _returnvalue 2)
        (`|SpawnActorFromClass` "/Game/FirstPerson/Blueprints/pickupitems/NailPickup.NailPickup_C" _returnvalue_2 "Undefined" "MultiplyWithRoot" null null)
        (else
          (`|SpawnActorFromClass` "/Game/FirstPerson/Blueprints/pickupitems/SawPickup.SawPickup_C" _returnvalue_2 "Undefined" "MultiplyWithRoot" null null)))))
  (if (> (`KismetMathLibrary.RandomFloatInRange` 0.0 100.0) 80.0)
    (`|SpawnActorFromClass` "/Game/FirstPerson/Blueprints/pickupitems/HealthPickup.HealthPickup_C" _returnvalue_2 "Undefined" "MultiplyWithRoot" null null))
  (if (> (`KismetMathLibrary.RandomFloatInRange` 0.0 100.0) 70.0)
    (`|SpawnActorFromClass` "/Game/FirstPerson/Blueprints/pickupitems/SawPickup.SawPickup_C" _returnvalue_2 "Undefined" "MultiplyWithRoot" null null)))

(fn `torchdeath`
  (bind _returnvalue (`KismetMathLibrary.RandomIntegerInRange` 1 3))
  (bind _returnvalue_2 (`KismetMathLibrary.MakeTransform` (`self.K2_GetActorLocation`)))
  (`|SpawnActorFromClass` "/Game/FirstPerson/Blueprints/pickupitems/AirPickup.AirPickup_C" _returnvalue_2 "Undefined" "MultiplyWithRoot" null null)
  (if (> (`KismetMathLibrary.RandomFloatInRange` 0.0 100.0) 60.0)
    (if (== _returnvalue 1)
      (`|SpawnActorFromClass` "/Game/FirstPerson/Blueprints/pickupitems/RebarPickup.RebarPickup_C" _returnvalue_2 "Undefined" "MultiplyWithRoot" null null)
      (elif (== _returnvalue 2)
        (`|SpawnActorFromClass` "/Game/FirstPerson/Blueprints/pickupitems/NailPickup.NailPickup_C" _returnvalue_2 "Undefined" "MultiplyWithRoot" null null)
        (else
          (`|SpawnActorFromClass` "/Game/FirstPerson/Blueprints/pickupitems/SawPickup.SawPickup_C" _returnvalue_2 "Undefined" "MultiplyWithRoot" null null)))))
  (if (> (`KismetMathLibrary.RandomFloatInRange` 0.0 100.0) 75.0)
    (`|SpawnActorFromClass` "/Game/FirstPerson/Blueprints/pickupitems/HealthPickup.HealthPickup_C" _returnvalue_2 "Undefined" "MultiplyWithRoot" null null)))

(fn `UserConstructionScript`)