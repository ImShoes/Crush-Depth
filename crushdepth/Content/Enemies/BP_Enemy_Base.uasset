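; Base enemy Blueprint providing attack, rifle equip and unequip, patrol route and movement speed actions.
; Attack plays a placeholder montage and calls OnAttackEnd when it completes or is interrupted.
; Equipping spawns a rifle on the hand socket; unequipping plays a montage whose notify destroys the rifle actor, calling OnUnEquipWeapon on completion.
; SetMovementSpeed maps idle, walk, jog and sprint states to max walk speed, and GetPatrolRoute exposes the assigned route.
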(event `/Game/Enemies/AI/BPI_EnemyAI.Attack`
  (`|PlayMontage` (`self.Mesh`) "/Game/AnimStarterPack/Montage_Place_Holder.Montage_Place_Holder"
    (:`OnCompleted`
      _)
    (:`OnInterrupted`
      _))
  (`self.OnAttackEnd`))

(event `/Game/Enemies/AI/BPI_EnemyAI.EquipWeapon`
  (bind _returnvalue (`|SpawnActorFromClass` "/Game/Enemies/BP_Rifle.BP_Rifle_C" (`self.GetTransform`) "Undefined" "MultiplyWithRoot" null null))
  (`self.K2_AttachToComponent` _returnvalue (`self.Mesh`) "hand_r_rifle_Socket" "SnapToTarget" "SnapToTarget" "SnapToTarget" true)
  (set `self.IsEquippingWeapon` true))

(event `/Game/Enemies/AI/BPI_EnemyAI.UnequipWeapon`
  (bind _notifyname (`|PlayMontage` (`self.Mesh`) "/Game/AnimStarterPack/Montage_Rifle_Idle.Montage_Rifle_Idle")
    (:`OnCompleted`
      (`self.OnUnEquipWeapon`))
    (:`OnNotifyBegin`
      (switch `name` _notifyname
        (:`Default`
          (`self.K2_DestroyActor` (`self.RifleActor`))
          (set `self.IsEquippingWeapon` false))))))

(fn `GetPatrolRoute`
  (returns (PatrolRoute :type "/Game/Enemies/AI/BP_PatrolRoute Object Reference"))
  (return (`self.PatrolRoute`)))

(fn `SetMovementSpeed`
  (params (Speed :type "/Game/Enemies/AI/Enums/E_MovementSpeed Enum" :default "NewEnumerator0"))
  (returns (SpeedValue :type "Float (double-precision)"))
  (bind _output_get (set `CharacterMovementComponent.MaxWalkSpeed` (select `/Game/Enemies/AI/Enums/E_MovementSpeed` Speed :`NewEnumerator1` 100.0 :`NewEnumerator2` 300.0 :`NewEnumerator3` 500.0 :!type "Float (single-precision)") (`self.CharacterMovement`)))
  (return _output_get))

(fn `UserConstructionScript`)